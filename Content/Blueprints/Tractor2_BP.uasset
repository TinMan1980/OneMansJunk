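; Trigger-driven tractor actor that comes to life and moves its mesh when the player enters its box.
; BP_PlayerCharacter entering starts audio, toggles headlights, colors the spheres' firefly dynamic material and plays a timeline lerp toward TractorLocation.
; VRPawn leaving reverses the timeline, then after a delay stops audio, blacks out the color and toggles headlights.
; Paired DoOnce gates reset each other to alternate both sequences.
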(event OnComponentBeginOverlap(Box)
  (params (OverlappedComponent :type Primitive%20Component%20Object%20Reference) (OtherActor :type Actor%20Object%20Reference) (OtherComp :type Primitive%20Component%20Object%20Reference) (OtherBodyIndex :type Integer) (bFromSweep :type Boolean) (SweepResult :type Hit%20Result%20Structure%20%28by%20ref%29))
  (Utilities|Casting|CastToBP_PlayerCharacter OtherActor)
  (Utilities|FlowControl|DoOnce false
    (:Completed
      (Components|Activation|Activate (Variables|Default|GetAudio) false)
      (|SetEmissiveColor)
      (Rendering|ToggleVisibility (Variables|Default|GetLeftHeadlight) false)
      (CallFunction|TractorMove)
      (CallFunction|Reverse1))))

(event OnComponentEndOverlap(Box)
  (params (OverlappedComponent :type Primitive%20Component%20Object%20Reference) (OtherActor :type Actor%20Object%20Reference) (OtherComp :type Primitive%20Component%20Object%20Reference) (OtherBodyIndex :type Integer))
  (Utilities|Casting|CastToVRPawn OtherActor)
  (Utilities|FlowControl|DoOnce false
    (:Completed
      (CallFunction|TractorReverse)
      (Utilities|FlowControl|Delay 1.0)
      (Components|Activation|Deactivate (Variables|Default|GetAudio))
      (|SetEmissiveColor_2)
      (Rendering|ToggleVisibility (Variables|Default|GetLeftHeadlight) false)
      (CallFunction|Reverse2))))

(event Custom|TractorMove
  (Variables|Default|SetIsMoved true)
  (bind _alpha (Timeline|Timeline_0 Play)
    (:Update
      (Transformation|SetRelativeLocation (Variables|Default|GetStaticMesh) (Math|Vector|Lerp(Vector) "0, 0, 0" (Variables|Default|GetTractorLocation) _alpha) false false))))

(event Custom|TractorReverse
  (Variables|Default|SetIsMoved false)
  (bind _alpha (Timeline|Timeline_0 Reverse)
    (:Update
      (Transformation|SetRelativeLocation (Variables|Default|GetStaticMesh) (Math|Vector|Lerp(Vector) "0, 0, 0" (Variables|Default|GetTractorLocation) _alpha) false false))))

(event Custom|Reverse1
  (Utilities|FlowControl|DoOnce false) ; enters at Reset
)

(event Custom|Reverse2
  (Utilities|FlowControl|DoOnce false) ; enters at Reset
)

(event EventBeginPlay
  (Utilities|FlowControl|DoOnce false
    (:Completed
      (Rendering|ToggleVisibility (Variables|Default|GetLeftHeadlight) false)
      (Components|Activation|Deactivate (Variables|Default|GetAudio)))))

(fn ConstructionScript
  (bind _returnvalue (Rendering|Material|CreateDynamicMaterialInstance (Variables|Default|GetSphere) 0 "/Game/Materials/NewFirefly_MAT.NewFirefly_MAT" "None" :!class /Script/Engine.PrimitiveComponent))
  (bind _output_get (Variables|Components|SetDMI _returnvalue))
  (bind _returnvalue_2 (Rendering|Material|CreateDynamicMaterialInstance (Variables|Default|GetSphere1) 0 _output_get "None" :!class /Script/Engine.PrimitiveComponent))
  (Variables|Components|SetDMI _returnvalue_2))