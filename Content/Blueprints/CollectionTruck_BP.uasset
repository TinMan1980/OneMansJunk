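; CollectionTruck_BP is a collection truck that turns dropped-in pickup items into cash.
; When a PickUpItem_BP overlaps its Box, the truck adds the item's AddAmout to CurrentCash, then destroys the item after a two-second delay.
; AddValue and SubtractValue events adjust the total, which Tick writes to the CashTotal text every frame.
; A Collect function simply returns its input and is not called in this graph.
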(event OnComponentBeginOverlap(Box)
  (params (OverlappedComponent :type Primitive%20Component%20Object%20Reference) (OtherActor :type Actor%20Object%20Reference) (OtherComp :type Primitive%20Component%20Object%20Reference) (OtherBodyIndex :type Integer) (bFromSweep :type Boolean) (SweepResult :type Hit%20Result%20Structure%20%28by%20ref%29))
  (bind _aspick_up_item_bp (Utilities|Casting|CastToPickUpItem_BP OtherActor))
  (CallFunction|AddValue (Variables|/Game/Blueprints/Treasure_BP/PickUpItem_BP.PickUpItem_BP_C|GetAdd%20Amout _aspick_up_item_bp))
  (Utilities|FlowControl|Delay 2.0)
  (Actor|DestroyActor _aspick_up_item_bp))

(event Custom|AddValue
  (params (ItemValue :type Integer))
  (Variables|Default|SetCurrentCash (+ ItemValue (Variables|Default|GetCurrentCash))))

(event Custom|SubtractValue
  (params (Item%20Value :type Integer))
  (Variables|Default|SetCurrentCash (- (Variables|Default|GetCurrentCash) Item%20Value)))

(event EventBeginPlay)

(event Collision|EventActorBeginOverlap
  (params (OtherActor :type Actor%20Object%20Reference)))

(event EventTick
  (params (DeltaSeconds :type Float%20%28single-precision%29))
  (Rendering|Components|TextRender|SetText (Variables|Default|GetCashTotal) (Utilities|Text|ToText(Integer) (Variables|Default|GetCurrentCash))))

(fn ConstructionScript)

(fn Collect
  (params (ItemValue :type Integer))
  (return ItemValue))