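; Door Blueprint with a grabbable lever handle and a Timeline that slides the door mesh.
; A looping timer, re-set every Tick, drives LeverActions to pitch the handle by the Arrow-to-Sphere X offset within a clamp; grab and drop reset both.
; ChangeLeverPulled plays the Timeline when IsMoved and Box overlaps Sphere1, reversing when IsMoved is false.
; The Timeline lerps relative location from zero to the world location cached at BeginPlay.
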(event OnGrabbed(GrabComponent)
  (Utilities|FlowControl|Delay 1.0)
  (Transformation|SetWorldRotation (Variables|Default|GetHandle) (Math|Rotator|MakeRotator 0.0 0.0 0.0) false false)
  (Transformation|SetWorldLocation (Variables|Default|GetSphere) (Transformation|GetWorldLocation (Variables|Default|GetArrow)) false false))

(event OnDropped(GrabComponent)
  (Transformation|SetWorldRotation (Variables|Default|GetHandle) (Math|Rotator|MakeRotator 0.0 0.0 0.0) false false)
  (Transformation|SetWorldLocation (Variables|Default|GetSphere) (Transformation|GetWorldLocation (Variables|Default|GetArrow)) false false))

(event Custom|DoorLocation
  (Variables|Default|SetDoorLocationVector (Transformation|GetWorldLocation (Variables|Debug|GetStaticMeshComponent))))

(event Custom|Change%20Lever%20Pulled
  (if (Variables|Default|GetIsMoved)
    (if (Class|PrimitiveComponent|IsOverlappingComponent (Variables|Default|GetBox) (Variables|Default|GetSphere1))
      (Utilities|FlowControl|DoOnce false :!label _label
        (:Completed
          (Variables|Default|SetIsMoved true)
          (bind _alpha (Timeline|Timeline Play)
            (:Update
              (Transformation|SetRelativeLocation (Variables|Debug|GetStaticMeshComponent) (Math|Vector|Lerp(Vector) "0, 0, 0" (Variables|Default|GetDoorLocationVector) _alpha) false false)))))
      (else
        (goto _label Reset)))
    (else
      (Variables|Default|SetIsMoved false)
      (Timeline|Timeline Reverse))))

(event Custom|LeverTimer
  (CallFunction|LeverActions))

(event EventBeginPlay
  (Utilities|Time|SetTimerbyEvent (delegate Custom|DoorLocation) 0.0))

(event Collision|EventActorBeginOverlap
  (params (OtherActor :type Actor%20Object%20Reference)))

(event EventTick
  (params (DeltaSeconds :type Float%20%28single-precision%29))
  (Utilities|Time|SetTimerbyEvent (delegate Custom|LeverTimer) 0.1 true))

(fn ConstructionScript)

(fn LeverActions
  (bind _handle (Variables|Default|GetHandle))
  (bind _returnvalue (Transformation|GetWorldRotation _handle))
  (Utilities|FlowControl|Sequence
    (:then_0
      (Transformation|SetWorldRotation _handle (Math|Rotator|MakeRotator (.roll _returnvalue) (Math|Float|Clamp(Float) (+ (.pitch _returnvalue) (.x (- (Transformation|GetWorldLocation (Variables|Default|GetArrow)) (Transformation|GetWorldLocation (Variables|Default|GetSphere))))) -25.0 0.0) (.yaw _returnvalue)) false false))))