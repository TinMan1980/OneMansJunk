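; GarageDoor_BP is a garage door actor with a grabbable handle driven by a GrabComponent.
; Every tick it adds the world X offset from Sphere to Arrow to the Handle's pitch, clamped to a narrow range.
; Dropping resets the Handle's rotation and snaps Sphere back to Arrow, as does grabbing after a short delay.
; A per-tick Box overlap check against Sphere1 has no action attached.
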(event OnGrabbed(GrabComponent)
  (Utilities|FlowControl|Delay 1.0)
  (Transformation|SetWorldRotation (Variables|Default|GetHandle) (Math|Rotator|MakeRotator 0.0 0.0 0.0) false false)
  (Transformation|SetWorldLocation (Variables|Default|GetSphere) (Transformation|GetWorldLocation (Variables|Default|GetArrow)) false false))

(event OnDropped(GrabComponent)
  (Transformation|SetWorldRotation (Variables|Default|GetHandle) (Math|Rotator|MakeRotator 0.0 0.0 0.0) false false)
  (Transformation|SetWorldLocation (Variables|Default|GetSphere) (Transformation|GetWorldLocation (Variables|Default|GetArrow)) false false))

(event EventBeginPlay)

(event Collision|EventActorBeginOverlap
  (params (OtherActor :type Actor%20Object%20Reference)))

(event EventTick
  (params (DeltaSeconds :type Float%20%28single-precision%29))
  (bind _handle (Variables|Default|GetHandle))
  (bind _returnvalue (Transformation|GetWorldRotation _handle))
  (Utilities|FlowControl|Sequence
    (:then_0
      (Transformation|SetWorldRotation _handle (Math|Rotator|MakeRotator (.roll _returnvalue) (Math|Float|Clamp(Float) (+ (.pitch _returnvalue) (.x (- (Transformation|GetWorldLocation (Variables|Default|GetArrow)) (Transformation|GetWorldLocation (Variables|Default|GetSphere))))) -25.0 0.0) (.yaw _returnvalue)) false false))
    (:then_1
      (if (Class|PrimitiveComponent|IsOverlappingComponent (Variables|Default|GetBox) (Variables|Default|GetSphere1))
        _))))

(fn ConstructionScript)