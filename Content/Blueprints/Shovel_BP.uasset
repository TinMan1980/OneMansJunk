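; Shovel Blueprint that digs into procedural terrain wherever its tip points.
; Every Tick, a short Visibility line trace runs forward from the Arrow component, looking for a ProcTerrain_BP.
; While it hits, a digging sound plays at the impact point each frame, and a brief Delay throttles the calls to AlterTerrain that deform the terrain.
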(event EventBeginPlay)

(event Collision|EventActorBeginOverlap
  (params (OtherActor :type Actor%20Object%20Reference)))

(event EventTick
  (params (DeltaSeconds :type Float%20%28single-precision%29))
  (bind _arrow (Variables|Default|GetArrow))
  (bind _returnvalue (Transformation|GetWorldLocation _arrow))
  (bind _outhit (Collision|LineTraceByChannel _returnvalue (+ _returnvalue (* (Math|Vector|GetForwardVector _arrow) 1e+02)) "TraceTypeQuery1" false 0 "None"))
  (if (Utilities|IsValid (.HitActor (Collision|BreakHitResult _outhit)))
    (bind _asproc_terrain_bp (Utilities|Casting|CastToProcTerrain_BP (.HitActor (Collision|BreakHitResult _outhit))))
    (Audio|PlaySoundatLocation "/Game/Sounds/Digging_Cue.Digging_Cue" (.ImpactPoint (Collision|BreakHitResult _outhit)) "0, 0, 0" 1.0 1.0 0.0 0 0 0 0)
    (Utilities|FlowControl|Delay 0.2)
    (Default|AlterTerrain _asproc_terrain_bp (.ImpactPoint (Collision|BreakHitResult _outhit)))))

(fn ConstructionScript)