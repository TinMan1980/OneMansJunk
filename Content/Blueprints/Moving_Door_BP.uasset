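; Moving door actor that slides its static mesh vertically on OpenDoor and CloseDoor events, which nothing in this Blueprint calls.
; BeginPlay caches the mesh's world location, and OpenDoor eases it to that point plus ZOffset over MoveSpeed seconds using MoveComponentTo.
; CloseDoor subtracts ZOffset from the current location rather than returning to the cached start.
; Both moves pass world-space locations as relative targets.
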(event EventBeginPlay
  (Variables|Default|SetStarting%20Location (Transformation|GetWorldLocation (Variables|Debug|GetStaticMeshComponent))))

(event Collision|EventActorBeginOverlap
  (params (OtherActor :type Actor%20Object%20Reference)))

(event EventTick
  (params (DeltaSeconds :type Float%20%28single-precision%29)))

(event EventCloseDoor
  (bind _staticmeshcomponent (Variables|Debug|GetStaticMeshComponent))
  (Components|MoveComponentTo _staticmeshcomponent (- (Transformation|GetWorldLocation _staticmeshcomponent) (Math|Vector|MakeVector 0.0 0.0 (Variables|Default|GetZ_Offset))) "0, 0, 0" true true (Variables|Default|GetMoveSpeed) false))

(event EventOpenDoor
  (Components|MoveComponentTo (Variables|Debug|GetStaticMeshComponent) (+ (Variables|Default|GetStarting%20Location) (Math|Vector|MakeVector 0.0 0.0 (Variables|Default|GetZ_Offset))) "0, 0, 0" true true (Variables|Default|GetMoveSpeed) false))

(fn ConstructionScript)