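; Level-streaming trigger actor that swaps sublevels when a Shovel_BP overlaps its box.
; The overlap blocking-loads the visible level at LevelInt in the Level array, then unloads CurrentLevel after a fixed delay.
; It then records the loaded level as CurrentLevel and calls SwitchLevel with a fixed index, setting which level loads on the next overlap.
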(event OnComponentBeginOverlap(Box)
  (params (OverlappedComponent :type Primitive%20Component%20Object%20Reference) (OtherActor :type Actor%20Object%20Reference) (OtherComp :type Primitive%20Component%20Object%20Reference) (OtherBodyIndex :type Integer) (bFromSweep :type Boolean) (SweepResult :type Hit%20Result%20Structure%20%28by%20ref%29))
  (bind _level (Variables|Default|GetLevel))
  (bind _levelint (Variables|Default|GetLevelInt))
  (bind _output (Utilities|Array|Get(acopy) _level _levelint))
  (Utilities|Casting|CastToShovel_BP OtherActor)
  (Class|GameplayStatics|LoadStreamLevelbySoftObjectPtr _output true true)
  (Utilities|FlowControl|Delay 2e+01)
  (Class|GameplayStatics|UnloadStreamLevelbySoftObjectPtr (Variables|Default|GetCurrentLevel) false)
  (Variables|Default|SetCurrentLevel _output)
  (CallFunction|SwitchLevel 1))

(event Custom|SwitchLevel
  (params (selection :type Integer))
  (Variables|Default|SetLevelInt selection))

(event EventBeginPlay)

(event Collision|EventActorBeginOverlap
  (params (OtherActor :type Actor%20Object%20Reference)))

(event EventTick
  (params (DeltaSeconds :type Float%20%28single-precision%29)))

(fn ConstructionScript)