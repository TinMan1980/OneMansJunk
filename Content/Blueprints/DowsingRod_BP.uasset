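; Dowsing rod actor that signals nearby PickUpItem_BP actors through left-hand haptics and rod movement.
; Detection is active only while GrabLeft is held and relies on Capsule overlaps.
; Overlap begin starts a looping haptic and plays the RodMovement timeline to yaw the rod outward.
; Overlap end replays the haptic unlooped and reverses the timeline.
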(event OnGrabbed(GrabLeft)
  (Variables|Default|SetFindEnabled true))

(event OnDropped(GrabLeft)
  (Variables|Default|SetFindEnabled false))

(event OnComponentBeginOverlap(Capsule)
  (params (OverlappedComponent :type Primitive%20Component%20Object%20Reference) (OtherActor :type Actor%20Object%20Reference) (OtherComp :type Primitive%20Component%20Object%20Reference) (OtherBodyIndex :type Integer) (bFromSweep :type Boolean) (SweepResult :type Hit%20Result%20Structure%20%28by%20ref%29))
  (if (Variables|Default|GetFindEnabled)
    (Utilities|Casting|CastToPickUpItem_BP OtherActor)
    ;[0.03434 0.03434 0.03434] Play Haptic Effect
    (Class|PlayerController|PlayHapticEffect (Game|GetPlayerController 0) "/Game/Blueprints/Haptics/Dowsing_Curve.Dowsing_Curve" "Left" 1.0 true)
    (CallFunction|MoveDowsingRod)))

(event OnComponentEndOverlap(Capsule)
  (params (OverlappedComponent :type Primitive%20Component%20Object%20Reference) (OtherActor :type Actor%20Object%20Reference) (OtherComp :type Primitive%20Component%20Object%20Reference) (OtherBodyIndex :type Integer))
  (if (Variables|Default|GetFindEnabled)
    (Utilities|Casting|CastToPickUpItem_BP OtherActor)
    (Class|PlayerController|PlayHapticEffect (Game|GetPlayerController 0) "/Game/Blueprints/Haptics/Dowsing_Curve.Dowsing_Curve" "Left" 1.0 false)
    (CallFunction|Reverse)))

(event Custom|MoveDowsingRod
  (bind _newtrack_0 (Timeline|RodMovement PlayFromStart)
    (:Update
      (Transformation|SetRelativeRotation (Variables|Default|GetRod) (Math|Rotator|MakeRotator 0.0 0.0 (Math|Float|Lerp 0.0 25.0 _newtrack_0)) false false))))

(event Custom|Reverse
  (bind _newtrack_0 (Timeline|RodMovement Reverse)
    (:Update
      (Transformation|SetRelativeRotation (Variables|Default|GetRod) (Math|Rotator|MakeRotator 0.0 0.0 (Math|Float|Lerp 0.0 25.0 _newtrack_0)) false false))))

(event EventBeginPlay)

(event Collision|EventActorBeginOverlap
  (params (OtherActor :type Actor%20Object%20Reference)))

(event EventTick
  (params (DeltaSeconds :type Float%20%28single-precision%29)))

(fn ConstructionScript)