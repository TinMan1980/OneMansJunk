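; ProcTerrain_BP is a deformable procedural terrain actor that copies a static mesh into a procedural mesh with collision and a landscape material.
; BeginPlay caches the mesh's geometry, recalculates normals and tangents after a short delay, then builds the section.
; AlterTerrain offsets vertices within a radius of an impact point by a depth vector, updating the section per changed vertex.
; A shoot input toggles that depth between digging and raising.
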(event Custom|GenerateMeash
  (Class|ProceduralMeshComponent|CreateMeshSectionLinearColor (Variables|Default|GetTerrain) 0 (Variables|Default|GetVertices) (Variables|Default|GetTriangles) (Variables|Default|GetNormals) (Variables|Default|GetUVs) 0 0 0 0 (Variables|Default|GetTangents) true false))

(event Custom|AlterTerrain
  (params (Impact%20Point :type Vector))
  (for (_array_element _array_index) (Variables|Default|GetVertices)
    (if (< (Math|Vector|VectorLength (- _array_element Impact%20Point)) (Variables|Default|GetRadius))
      (Utilities|Array|SetArrayElem (Variables|Default|GetVertices) _array_index (- _array_element (Variables|Default|GetDepth)))
      (Class|ProceduralMeshComponent|UpdateMeshSectionLinearColor (Variables|Default|GetTerrain) 0 (Variables|Default|GetVertices) (Variables|Default|GetNormals) 0 0 0 0 0 0 true))))

(event Input|EnhancedActionEvents|EnhancedInputActionIA_Shoot_Right
  (params (ActionValue :type Boolean) (ElapsedSeconds :type Float%20%28double-precision%29) (TriggeredSeconds :type Float%20%28double-precision%29) (InputAction :type Input%20Action%20Object%20Reference :default "/Game/VRTemplate/Input/Actions/IA_Shoot_Right.IA_Shoot_Right"))
  (:Triggered
    ;[1 1 1] Change between dig and raise terrain not needed in game
    (Utilities|FlowControl|FlipFlop
      (:A
        (Variables|Default|SetDepth "0, 0,20.000000"))
      (:B
        (Variables|Default|SetDepth "0, 0,-20.000000")))))

(event EventBeginPlay
  (Input|EnableInput (Game|GetPlayerController 0))
  (Rendering|Material|SetMaterial (Variables|Default|GetTerrain) 0 "/Game/ProcTerrain/Landscape_MAT.Landscape_MAT")
  (bind (_vertices _triangles _normals _uvs) (Class|KismetProceduralMeshLibrary|GetSectionfromStaticMesh (Variables|/Script/Engine.StaticMeshComponent|GetStaticMesh (Variables|Default|GetBaseMesh))))
  (Variables|Default|SetVertices _vertices)
  (Variables|Default|SetTriangles _triangles)
  (Variables|Default|SetUVs _uvs)
  (Utilities|FlowControl|Delay 0.2)
  (bind (_normals_2 _tangents) (Class|KismetProceduralMeshLibrary|CalculateTangentsforMesh (Variables|Default|GetVertices) (Variables|Default|GetTriangles) (Variables|Default|GetUVs)))
  (Variables|Default|SetNormals _normals_2)
  (Variables|Default|SetTangents _tangents)
  (Class|ProceduralMeshComponent|UpdateMeshSectionLinearColor (Variables|Default|GetTerrain) 0 (Variables|Default|GetVertices) (Variables|Default|GetNormals) (Variables|Default|GetUVs) 0 0 0 0 (Variables|Default|GetTangents) true)
  (CallFunction|GenerateMeash))

(fn ConstructionScript)