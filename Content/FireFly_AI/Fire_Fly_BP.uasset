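; Firefly actor that wanders inside the FlyingAi_Manager's box and plays a mosquito sound when a VRPawn overlaps its sphere.
; BeginPlay randomizes light intensity, color, material glow and timeline speed and length, then starts wandering.
; A timeline lerps location and rotation toward a random box point, picking another when finished.
; A looping timer line-traces ahead; static mesh hits stop movement, randomize rotation and restart wandering.
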(event OnComponentBeginOverlap(Sphere1)
  (params (OverlappedComponent :type Primitive%20Component%20Object%20Reference) (OtherActor :type Actor%20Object%20Reference) (OtherComp :type Primitive%20Component%20Object%20Reference) (OtherBodyIndex :type Integer) (bFromSweep :type Boolean) (SweepResult :type Hit%20Result%20Structure%20%28by%20ref%29))
  (Utilities|Casting|CastToVRPawn OtherActor)
  (Audio|PlaySound2D "/Game/Sounds/Mosquito_Cue.Mosquito_Cue" 1.0 1.0 0.0 0 0))

(event Custom|Wander
  (|Flyingmovement))

(event Custom|Trace
  (|objectavoidance))

(event EventBeginPlay
  (|runtimeevents))

(fn ConstructionScript
  (bind _returnvalue (Rendering|Material|CreateDynamicMaterialInstance (Variables|Default|Getbody) 0 "/Game/Materials/NewFirefly_MAT.NewFirefly_MAT" "None" :!class /Script/Engine.PrimitiveComponent))
  (Variables|Default|SetDMI _returnvalue))

(event Custom|Stop%20movement
  ;[1 1 1] Flying movement
  (bind _movementalpha (Timeline|Movement Stop)
    (:Update
      (Transformation|SetActorLocation (Math|Vector|Lerp(Vector) (Transformation|GetActorLocation) (Variables|Default|GetRandomPoint) _movementalpha) false false)
      (Transformation|SetActorRotation (Math|Rotator|Lerp(Rotator) (Transformation|GetActorRotation) (Math|Rotator|FindLookatRotation (Transformation|GetActorLocation) (Variables|Default|GetRandomPoint)) _movementalpha)))
    (:Finished
      (CallFunction|Wander))))