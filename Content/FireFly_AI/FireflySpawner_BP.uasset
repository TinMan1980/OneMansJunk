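; Firefly spawner actor that populates a box volume with Fire_Fly_BP actors when play begins.
; On BeginPlay it loops FireflyNumber times, spawning each firefly at a random point inside the box centred on the spawner, at a small uniform scale.
; The construction script sizes the Box component from InBoxExtent, so the visible volume matches the spawn area.
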(event EventBeginPlay
  (for _index (range 0 (- (Variables|Default|Getfirefly%20number) 1))
    (Game|SpawnActorfromClass "/Game/FireFly_AI/Fire_Fly_BP.Fire_Fly_BP_C" (Math|Transform|MakeTransform (Math|Random|RandomPointinBoundingBox (Transformation|GetActorLocation) (Variables|Default|GetIn%20Box%20Extent)) "0, 0, 0" (Math|Vector|MakeVector 0.04 0.04 0.04)) "Undefined" 0 0)))

(fn ConstructionScript
  (Components|Box|SetBoxExtent (Variables|Default|GetBox) (Variables|Default|GetIn%20Box%20Extent) true))