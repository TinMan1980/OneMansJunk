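; ItemSpawn_BP is a box-shaped spawner that scatters items over procedural terrain one second after BeginPlay.
; The construction script sizes the Box from InBoxExtent, and SpawnItems runs SpawnNum downward traces between separately randomized points, so rays slant.
; Only hits on ProcTerrain_BP spawn an actor, picked randomly from the first three ItemsToSpawn classes and sunk slightly below the hit point.
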(event Custom|SpawnItems
  (bind _returnvalue (Transformation|GetActorLocation))
  (bind _in_box_extent (Variables|Default|GetIn%20Box%20Extent))
  (bind _returnvalue_2 (Math|Random|RandomPointinBoundingBox _returnvalue _in_box_extent))
  (for _index (range 0 (Variables|Default|GetSpawnNum))
    (bind _outhit (Collision|LineTraceByChannel _returnvalue_2 (- _returnvalue_2 "0, 0,2000.000000") "TraceTypeQuery2" true 0 "ForOneFrame"))
    (Utilities|Casting|CastToProcTerrain_BP (.HitActor (Collision|BreakHitResult _outhit)))
    (Game|SpawnActorfromClass (Utilities|Array|Get(acopy) (Variables|Default|GetItemsToSpawn) (Math|Random|RandomIntegerinRange 0 2)) (Math|Transform|MakeTransform (- (.Location (Collision|BreakHitResult _outhit)) "0.0,0.0,20.000000") "0, 0, 0" (Variables|Default|GetSpawn%20Transform%20Scale)) "Undefined" 0 0)))

(event EventBeginPlay
  (Utilities|FlowControl|Delay 1.0)
  (CallFunction|SpawnItems))

(fn ConstructionScript
  (Components|Box|SetBoxExtent (Variables|Default|GetBox) (Variables|Default|GetIn%20Box%20Extent) true))